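; BP_Terrain is a terrain tile in a Crossy Road-style game that triggers spawning of further terrain as the player advances.
; When BP_ThirdPersonCharacter enters TriggerZone, the tile calls TerrainSpawner to spawn terrain at its spawn point, then destroys itself.
; RandomizeTerrain, not called within this Blueprint, sets the Road mesh from a random index into six terrain types, but its range never reaches Water.
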(event OnComponentBeginOverlap(TriggerZone)
  (params (OverlappedComponent :type Primitive%20Component%20Object%20Reference) (OtherActor :type Actor%20Object%20Reference) (OtherComp :type Primitive%20Component%20Object%20Reference) (OtherBodyIndex :type Integer) (bFromSweep :type Boolean) (SweepResult :type Hit%20Result%20Structure%20%28by%20ref%29))
  (Utilities|Casting|CastToBP_ThirdPersonCharacter OtherActor)
  (Default|SpawnTerrainatSpawnPoint (Variables|Default|GetTerrainSpawner))
  (Actor|DestroyActor))

(event Collision|EventActorBeginOverlap
  (params (OtherActor :type Actor%20Object%20Reference)))

(fn ConstructionScript)

(fn RandomizeTerrain
  (Utilities|FlowControl|Sequence
    (:then_1
      (Variables|Default|SetRandomizer (Math|Random|RandomIntegerinRange 0 4)))
    (:then_2
      (bind _output_get (Variables|Default|SetMesh_Name (Utilities|Select :Index (Variables|Default|GetRandomizer) :Option%200 "/Game/CrossyRoad/Mesh/Highway.Highway" :Option%201 "/Game/CrossyRoad/Mesh/Dirt_Road.Dirt_Road" :Option%202 "/Game/CrossyRoad/Mesh/Grass_Flowers.Grass_Flowers" :Option%203 "/Game/CrossyRoad/Mesh/Road.Road" :Option%204 "/Game/CrossyRoad/Mesh/Street.Street" :Option%205 "/Game/CrossyRoad/Mesh/Water.Water")))
      (Components|StaticMesh|SetStaticMesh (Variables|Components|GetRoad) _output_get))))