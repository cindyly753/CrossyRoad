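; Terrain spawner for a Crossy Road-style game that builds a chain of randomized BP_Terrain pieces when play begins.
; The first piece spawns at the player pawn, and each later one at the newest piece's SpawnPoint.
; Each piece receives a reference to the spawner and randomizes itself.
; A BP_Truck spawns alongside every piece at a randomized Y, as the Highway mesh check is unconnected.
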(event EventBeginPlay
  (CallFunction|SpawnInitialTerrain))

(event Collision|EventActorBeginOverlap
  (params (OtherActor :type Actor%20Object%20Reference)))

(event EventTick
  (params (DeltaSeconds :type Float%20%28single-precision%29)))

(fn ConstructionScript)

(fn SpawnTerrain
  (params (SpawnLocation :type Vector))
  (bind (_x _y _z) (Math|Vector|BreakVector SpawnLocation))
  (Utilities|FlowControl|Sequence
    (:then_0
      (bind _returnvalue (Game|SpawnActorfromClass "/Game/CrossyRoad/Blueprints/BP_Terrain.BP_Terrain_C" (Math|Transform|MakeTransform SpawnLocation "0, 0, 0" "1.000000,1.000000,1.000000") "Undefined" 0 0))
      (bind _output_get (Variables|Default|SetNewestTerrain _returnvalue))
      (Variables|/Game/CrossyRoad/Blueprints/BP_Terrain.BP_Terrain_C|SetTerrainSpawner _output_get self)
      (Default|RandomizeTerrain _output_get))
    (:then_1
      (if true
        (Game|SpawnActorfromClass "/Game/CrossyRoad/Blueprints/BP_Truck.BP_Truck_C" (Math|Transform|MakeTransform (Math|Vector|MakeVector _x (+ (* (Math|Random|RandomFloatinRange 1.0 4.0) _y) -3e+03) _z) "0, 0, 0" "1.000000,1.000000,1.000000") "Undefined" 0 0)))))

(fn SpawnTerrainatSpawnPoint
  (CallFunction|SpawnTerrain (Transformation|GetWorldLocation (Variables|/Game/CrossyRoad/Blueprints/BP_Terrain.BP_Terrain_C|GetSpawnPoint (Variables|Default|GetNewestTerrain)))))

(fn SpawnInitialTerrain
  (for _index (range 0 20)
    (Utilities|IsValid (Variables|Default|GetNewestTerrain)
      (:Is%20Valid
        (CallFunction|SpawnTerrainatSpawnPoint))
      (:Is%20Not%20Valid
        (CallFunction|SpawnTerrain (Transformation|GetActorLocation (Game|Player|GetPlayerPawn 0)))))))

(fn EqualMesh)